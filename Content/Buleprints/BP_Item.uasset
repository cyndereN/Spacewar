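; BP_Item is a pickup that grants a speed, health, damage or score bonus to an overlapping BP_AI or BP_SpaceShip.
; SetColor rolls a type weighted toward score, tints a dynamic material to match and plays a scale-in timeline.
; Overlap applies that type's effect, calls BufferDisapper for speed and damage or updates WBP_HP_Local for score, then calls OnDeath.
; SpawnExplosion emits particles in the item's color.
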(event `self.ReceiveBeginPlay`
  (bind _foundwidgets (`WidgetBlueprintLibrary.GetAllWidgetsOfClass` "/Game/Buleprints/Widget/WBP_HP_Local.WBP_HP_Local_C"))
  (set `self.WBP_HP` (`|GetArrayItem` _foundwidgets)))

(event `self.SetColor`
  (bind _returnvalue (`KismetMathLibrary.RandomIntegerInRange` 0 3))
  (bind _returnvalue_2 (select `int` (`self.BodyColorIndex`) :`0` (struct :`R` 1.0 :`G` 0.538341 :`A` 1.0) :`1` (struct :`G` 1.0 :`A` 1.0) :`2` (struct :`R` 1.0 :`A` 1.0) :`3` (struct :`A` 1.0) :!type "LinearColor Structure"))
  (set `self.BodyColorIndex` (`KismetMathLibrary.SelectInt` 3 _returnvalue (== _returnvalue 1)))
  (bind _returnvalue_3 (`KismetMaterialLibrary.CreateDynamicMaterialInstance` "/Game/SpaceshipBattle/Materials/M_Base_Ship.M_Base_Ship"))
  (`MaterialInstanceDynamic.SetVectorParameterValue` _returnvalue_3 "Color3" _returnvalue_2)
  (set `self.PrimaryColor` _returnvalue_2)
  (set `self.SecondryColor` _returnvalue_2)
  (`PrimitiveComponent.SetMaterial` (`self.EnemySM`) 0 _returnvalue_3)
  (bind (_direction _scale) (`Timeline|SpawnScaleTimeLine`)
    (:`Update`
      (`self.SetActorScale3D` (`KismetMathLibrary.Conv_DoubleToVector` _scale)))))

(event `self.SpawnExplosion`
  (bind _returnvalue (`GameplayStatics.SpawnEmitterAtLocation` "/Game/ParticleSystem/PS_Explosion.PS_Explosion" (`self.K2_GetActorLocation`)))
  (`FXSystemComponent.SetColorParameter` _returnvalue "PrimaryColor" (`self.PrimaryColor`))
  (`FXSystemComponent.SetColorParameter` _returnvalue "SecondryColor" (`self.SecondryColor`)))

(event `self.ReceiveActorBeginOverlap`
  (params (OtherActor :type "Actor Object Reference"))
  (bind _as_ai (`self.As AI`))
  (bind _as_bp_space_ship (`self.As BP Space Ship`))
  (bind _as_bp_space_ship_2 (`self.As BP Space Ship`))
  (bind _as_ai_2 (`self.As AI`))
  (bind _as_ai_3 (`self.As AI`))
  (bind _as_ai_4 (`self.As AI`))
  (bind _as_bp_space_ship_3 (`self.As BP Space Ship`))
  (bind _as_bp_space_ship_4 (`self.As BP Space Ship`))
  (bind _asbp_ai (cast `/Game/Buleprints/BP_AI` OtherActor)
    (:`then`
      (set `self.As AI` _asbp_ai)
      (switch `int` (`self.BodyColorIndex`)
        (:`0`
          (set `FloatingPawnMovement.MaxSpeed` 2400.0 (`/Game/Buleprints/BP_AI.FloatingPawnMovement` _as_ai_2))
          (`/Game/Buleprints/BP_AI.BufferDisapper` _as_ai_2 (`self.BodyColorIndex`))
          (`self.OnDeath`))
        (:`1`
          (set `/Game/Buleprints/BP_AI.HP` (`KismetMathLibrary.FMin` (+ (`/Game/Buleprints/BP_AI.HP` _as_ai_4) 40.0) 100.0) _as_ai_4)
          (`self.OnDeath`))
        (:`2`
          (set `/Game/Buleprints/BP_AI.Damage` 5.0 _as_ai)
          (`/Game/Buleprints/BP_AI.BufferDisapper` _as_ai (`self.BodyColorIndex`))
          (`self.OnDeath`))
        (:`3`
          (bind _output_get (set `/Game/Buleprints/BP_AI.Score` (+ (`/Game/Buleprints/BP_AI.Score` _as_ai_3) 50) _as_ai_3))
          (`/Game/Buleprints/Widget/WBP_Score.Get Score` (`|GetArrayItem` (`/Game/Buleprints/Widget/WBP_HP_Local.GetScoreArray` (`self.WBP_HP`)) (`/Game/Buleprints/BP_AI.BodyColorIndex` _as_ai_3)) _output_get)
          (`self.OnDeath`))))
    (:`CastFailed`
      (bind _asbp_space_ship (cast `/Game/Buleprints/BP_SpaceShip` OtherActor))
      (set `self.As BP Space Ship` _asbp_space_ship)
      (switch `int` (`self.BodyColorIndex`)
        (:`0`
          (set `SpaceShip.Speed` 3500.0 _as_bp_space_ship_2)
          (`/Game/Buleprints/BP_SpaceShip.BufferDisapper` _as_bp_space_ship_2 (`self.BodyColorIndex`))
          (`self.OnDeath`))
        (:`1`
          (set `/Game/Buleprints/BP_SpaceShip.HP` (`KismetMathLibrary.FMin` (+ (`/Game/Buleprints/BP_SpaceShip.HP` _as_bp_space_ship) 40.0) 100.0) _as_bp_space_ship)
          (`self.OnDeath`))
        (:`2`
          (set `/Game/Buleprints/BP_SpaceShip.Damage` 5.0 _as_bp_space_ship_4)
          (`/Game/Buleprints/BP_SpaceShip.BufferDisapper` _as_bp_space_ship_4 (`self.BodyColorIndex`))
          (`self.OnDeath`))
        (:`3`
          (bind _output_get_2 (set `/Game/Buleprints/BP_SpaceShip.Score` (+ (`/Game/Buleprints/BP_SpaceShip.Score` _as_bp_space_ship_3) 50) _as_bp_space_ship_3))
          (`/Game/Buleprints/Widget/WBP_Score.Get Score` (`/Game/Buleprints/Widget/WBP_HP_Local.TextBlock_Red` (`self.WBP_HP`)) _output_get_2)
          (`self.OnDeath`))))))

(fn `UserConstructionScript`)