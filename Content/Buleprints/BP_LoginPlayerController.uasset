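; Player controller for an online game that carries each player from pre-session lobby through match to game over.
; Ready, start, damage and death events relay through BP_LoginGameMode, with client-side events updating lobby, HP and end-screen widgets.
; Game start clears DefaultPawns and kicks off the first BP_EnemySpawn_Online.
; Helpers pick a session by matching build ID and compute a top-down aim rotation from the cursor's offset to screen center.
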(event `self.ReceiveBeginPlay`
  (set `self.Ready` false)
  (set `self.bShowMouseCursor` true)
  (set `self.Death` false))

(event `UpdateInfoOnClient`
  (params (UserName :type "Array of Text") (Ready :type "Array of Boolean"))
  (set `self.User Name` UserName)
  (set `self.ReadyArray` Ready)
  (`/Engine/EditorBlueprintResources/StandardMacros.IsValid` (`self.WBP_PreSession`)
    (:`Is Valid`
      (`PanelWidget.ClearChildren` (`/Game/Buleprints/Widget/WBP_PreSession.VerticalBox_List` (`self.WBP_PreSession`))))
    (:`Is Not Valid`
      (bind _returnvalue (`|CreateWidget` "/Game/Buleprints/Widget/WBP_PreSession.WBP_PreSession_C" self))
      (bind _output_get (set `self.WBP_PreSession` _returnvalue))
      (`UserWidget.AddToViewport` _output_get 0)
      (bind _verticalbox_list (`/Game/Buleprints/Widget/WBP_PreSession.VerticalBox_List` _output_get))
      (`PanelWidget.ClearChildren` _verticalbox_list)))
  (for (_array_element _array_index) (`self.User Name`)
    (bind _returnvalue_2 (`|CreateWidget` "/Game/Buleprints/Widget/WBP_PlayerItem.WBP_PlayerItem_C" null _array_element))
    (`/Game/Buleprints/Widget/WBP_PlayerItem.OnReady` _returnvalue_2 (`|GetArrayItem` (`self.ReadyArray`) _array_index))
    (`VerticalBox.AddChildToVerticalBox` _verticalbox_list _returnvalue_2)))

(event `ReadyOnServer`
  (params (Ready :type Boolean))
  (`self.ReadyOnMulticast` Ready))

(event `ReadyOnMulticast`
  (params (Ready :type Boolean))
  (set `self.Ready` Ready)
  (bind _asbp_login_game_mode (cast `/Game/Buleprints/BP_LoginGameMode` (`GameplayStatics.GetGameMode`)))
  (`/Game/Buleprints/BP_LoginGameMode.UpdateOnReady` _asbp_login_game_mode self (`self.Ready`)))

(event `VisibilityButtonOnServer`
  (params (WBP_Pre :type "/Game/Buleprints/Widget/WBP_PreSession Object Reference"))
  (`/Engine/EditorBlueprintResources/StandardMacros.IsValid` WBP_Pre
    (:`Is Valid`
      (`/Game/Buleprints/Widget/WBP_PreSession.Set StartGame` WBP_Pre))))

(event `OpenGameOnServer`
  (bind _asbp_login_game_mode (cast `/Game/Buleprints/BP_LoginGameMode` (`GameplayStatics.GetGameMode`)))
  (`/Game/Buleprints/BP_LoginGameMode.StartGameOnClient` _asbp_login_game_mode))

(event `OpenGameOnClient`
  (bind _wbp_presession (`self.WBP_PreSession`))
  (`WidgetBlueprintLibrary.SetInputMode_GameAndUIEx` self null "DoNotLock" false)
  (bind _outactors (`GameplayStatics.GetAllActorsOfClass` "/Script/Engine.DefaultPawn"))
  (for _array_element _outactors
    (`self.K2_DestroyActor` _array_element))
  (`/Engine/EditorBlueprintResources/StandardMacros.IsValid` _wbp_presession
    (:`Is Valid`
      (`Widget.RemoveFromParent` _wbp_presession)
      (bind _outactors_2 (`GameplayStatics.GetAllActorsOfClass` "/Game/Buleprints/BP_EnemySpawn_Online.BP_EnemySpawn_Online_C"))
      (`/Game/Buleprints/BP_EnemySpawn_Online.Custom Beginplay` (`|GetArrayItem` _outactors_2))
      (bind _returnvalue (`|CreateWidget` "/Game/Buleprints/Widget/WBP_HP.WBP_HP_C"))
      (bind _output_get (set `self.WBP_HP` _returnvalue))
      (`UserWidget.AddToViewport` _output_get 0))))

(event `ReceiveDamageUIOnServer`
  (params (HP :type "Float (double-precision)") (Index :type Integer) (`Damage Target` :type "Actor Object Reference"))
  (bind _asbp_login_game_mode (cast `/Game/Buleprints/BP_LoginGameMode` (`GameplayStatics.GetGameMode`)))
  (`/Game/Buleprints/BP_LoginGameMode.ReceiveDamageUIOnClient` _asbp_login_game_mode HP Index `Damage Target`))

(event `ReceiveDamage`
  (params (HP :type "Float (double-precision)") (Index :type Integer) (`Damage Target` :type "Actor Object Reference"))
  (`/Game/Buleprints/Widget/WBP_HP.Recieve Damage` (`self.WBP_HP`) HP Index `Damage Target`))

(event `DeathOnMulticast`
  (params (Death :type Boolean))
  (bind _output_get (set `self.Death` Death))
  (bind _asbp_login_game_mode (cast `/Game/Buleprints/BP_LoginGameMode` (`GameplayStatics.GetGameMode`)))
  (`/Game/Buleprints/BP_LoginGameMode.StopGameOnClient` _asbp_login_game_mode _output_get self))

(event `StopGameOnServer`
  (params (Death :type Boolean))
  (`self.DeathOnMulticast` Death))

(event `StopGameOnController`
  (params (Death :type Boolean))
  (bind _returnvalue (`|CreateWidget` "/Game/Buleprints/Widget/WBP_UserInterface.WBP_UserInterface_C" self true))
  (`UserWidget.AddToViewport` _returnvalue 0))

(fn `GetCurrentSession`
  (params (Array :type "Array of BlueprintSessionResult Structure"))
  (returns (Session :type "BlueprintSessionResult Structure"))
  (locals (Local :type "BlueprintSessionResult Structure"))
  (for _array_element Array
    (if (== (`AdvancedSessionsLibrary.GetCurrentUniqueBuildID`) (`AdvancedSessionsLibrary.GetUniqueBuildID` _array_element))
      (set `local.Local` _array_element)
      (break)))
  (return (`local.Local`)))

(fn `SetPlayerController`
  (returns (Output_Get :type "Rotator Structure"))
  (bind (_locationx _locationy) (`self.GetMousePosition` self))
  (bind (_returnvalue_roll _returnvalue_pitch _returnvalue_yaw) (`KismetMathLibrary.BreakRotator` (`KismetMathLibrary.FindLookAtRotation` (`KismetMathLibrary.Conv_Vector2DToVector` (/ (`WidgetLayoutLibrary.GetViewportSize`) 2.0)) (`KismetMathLibrary.Conv_Vector2DToVector` (`KismetMathLibrary.MakeVector2D` _locationx _locationy)))))
  (`/Engine/EditorBlueprintResources/StandardMacros.IsValid` self
    (:`Is Valid`
      (bind _output_get (set `self.Rotation` (`KismetMathLibrary.MakeRotator` _returnvalue_roll _returnvalue_pitch (+ _returnvalue_yaw 90.0))))
      (return _output_get))))

(fn `UserConstructionScript`)