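; BP_Bullet is a bullet actor that damages the actor it overlaps and then destroys itself.
; On BeginPlay it creates a dynamic material instance on BulletSM and tints it through the Color1 parameter using its Color variable.
; Overlaps with its DamageCauser are ignored; any other actor is passed to a custom ApplyDamage event, which applies BaseDamage and destroys the bullet.
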(event `self.ReceiveBeginPlay`
  (bind _bulletsm (`self.BulletSM`))
  (bind _returnvalue (`PrimitiveComponent.CreateDynamicMaterialInstance` _bulletsm 0 (`PrimitiveComponent.GetMaterial` _bulletsm 0) "None"))
  (`MaterialInstanceDynamic.SetVectorParameterValue` _returnvalue "Color1" (`self.Color`)))

(event `self.ReceiveActorBeginOverlap`
  (params (OtherActor :type "Actor Object Reference"))
  (if (not (== (`self.Damage Causer`) OtherActor))
    (`self.ApplyDamage` OtherActor (`self.Base Damage`) (`self.Damage Causer`))))

(event `ApplyDamage`
  (params (DamagedActor :type "Actor Object Reference") (BaseDamage :type "Float (double-precision)") (DamageCauser :type "Actor Object Reference"))
  (`GameplayStatics.ApplyDamage` DamagedActor BaseDamage null DamageCauser "/Script/Engine.DamageType")
  (`self.K2_DestroyActor` self))

(fn `UserConstructionScript`)