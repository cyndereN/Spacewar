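; BP_AI is an AI-controlled ship that fights nearby pawns, colored by its body color index.
; Looping timers drive sphere-trace targeting with bullet fire, random NavMesh wandering and backing away from close pawns.
; An item-seeking timer pauses movement timers when this AI is the closest AI to a detected item.
; Damage flows through server and multicast events to update HP widgets, award the attacker score and explode on death.
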(event `self.ReceiveBeginPlay`
  (`self.BeginOnServer`))

(event `BeginOnMulticast`
  (bind _returnvalue (select `int` (`self.BodyColorIndex`) :`0` (struct :`R` 1.0 :`A` 1.0) :`1` (struct :`G` 1.0 :`A` 1.0) :`2` (struct :`B` 1.0 :`A` 1.0) :`3` (struct :`R` 1.0 :`G` 1.0 :`A` 1.0) :!type "LinearColor Structure"))
  (`self.FindItems`)
  (`self.AIRandomMovement`)
  (`self.AIFarAwayMovement`)
  (bind _returnvalue_2 (`KismetMaterialLibrary.CreateDynamicMaterialInstance` "/Game/SpaceshipBattle/Materials/MI_Ship_Player.MI_Ship_Player"))
  (`MaterialInstanceDynamic.SetVectorParameterValue` _returnvalue_2 "Color3" _returnvalue)
  (set `self.PrimaryColor` _returnvalue)
  (`FXSystemComponent.SetColorParameter` (`self.Niagara`) "Color" (`self.PrimaryColor`))
  (set `self.SecondryColor` (select `int` (`self.BodyColorIndex`) :`0` (struct :`R` 1.0 :`G` 0.304093 :`B` 0.072683 :`A` 1.0) :`1` (struct :`R` 0.166862 :`G` 0.410326 :`B` 1.0 :`A` 1.0) :`2` (struct :`R` 0.480823 :`G` 1.0 :`B` 0.121041 :`A` 1.0) :`3` (struct :`R` 1.0 :`B` 0.179739 :`A` 1.0) :!type "LinearColor Structure"))
  (`PrimitiveComponent.SetMaterial` (`self.StaticMesh`) 0 _returnvalue_2)
  (`KismetSystemLibrary.K2_SetTimerDelegate` (delegate `GetTargetLocation`) 0.15 true)
  (`self.Get WBP_Main`))

(event `BeginOnServer`
  (`self.BeginOnMulticast`))

(event `GetTargetLocation`
  (bind _returnvalue (`self.K2_GetActorLocation`))
  (bind _pawn (`self.Pawn`))
  (bind _distance (`self.Distance`))
  (bind _pawn_2 (`self.Pawn`))
  (bind _distance_2 (`self.Distance`))
  (bind (_returnvalue_roll _returnvalue_pitch _returnvalue_yaw) (`KismetMathLibrary.BreakRotator` (`KismetMathLibrary.FindLookAtRotation` (`self.K2_GetActorLocation`) (`self.K2_GetActorLocation` (`BlueprintMapLibrary.Map_Find` (`self.Pawn`) (`.MinValue` (`KismetMathLibrary.MinOfFloatArray` (`self.Distance`))))))))
  (bind (_returnvalue_roll_2 _returnvalue_pitch_2 _returnvalue_yaw_2) (`KismetMathLibrary.BreakRotator` (`KismetMathLibrary.FindLookAtRotation` (`self.K2_GetActorLocation`) (`self.K2_GetActorLocation` (`BlueprintMapLibrary.Map_Find` (`self.Pawn`) (`.MaxValue` (`KismetMathLibrary.MaxOfFloatArray` (`self.Distance`))))))))
  (bind (_outhits _returnvalue_2) (`KismetSystemLibrary.SphereTraceMultiForObjects` _returnvalue (+ _returnvalue (0.0 0.0 10.0)) 3000.0 (`|MakeArray` "ObjectTypeQuery3" :!type "EObjectTypeQuery Enum")))
  (if _returnvalue_2
    (for _array_element _outhits
      (bind (_bblockinghit _binitialoverlap _time _distance_3 _location _impactpoint _normal _impactnormal _physmat _hitactor) (`GameplayStatics.BreakHitResult` _array_element))
      (bind _aspawn (cast `Pawn` _hitactor))
      (bind _returnvalue_3 (`KismetMathLibrary.Vector_Distance` _location (`self.K2_GetActorLocation` _aspawn)))
      (`KismetArrayLibrary.Array_Add` (`self.Distance`) _returnvalue_3)
      (`BlueprintMapLibrary.Map_Add` (`self.Pawn`) _returnvalue_3 _aspawn))
    (`self.K2_SetActorRotation` (`KismetMathLibrary.MakeRotator` 0.0 0.0 _returnvalue_yaw))
    (if (> (`.MaxValue` (`KismetMathLibrary.MaxOfFloatArray` (`self.Distance`))) 2000.0)
      (`self.K2_SetActorRotation` (`KismetMathLibrary.MakeRotator` 0.0 0.0 _returnvalue_yaw_2))
      (`self.Fire`)
      (else
        (`self.Fire`)))
    (set `self.LocalDistance` _distance_2)
    (set `self.LocalPawn` _pawn_2)
    (`KismetArrayLibrary.Array_Clear` _distance_2)
    (`BlueprintMapLibrary.Map_Clear` _pawn_2)
    (else
      (set `self.LocalDistance` _distance)
      (set `self.LocalPawn` _pawn)
      (`KismetArrayLibrary.Array_Clear` _distance)
      (`BlueprintMapLibrary.Map_Clear` _pawn))))

(event `BufferDisapper`
  (params (Int :type Integer))
  (`self.BufferDisapperOnMulticast` Int))

(event `BufferDisapperOnMulticast`
  (params (Int :type Integer))
  (switch `int` Int
    (:`0`
      ;[1 1 1] Buffer持续时间
      (`KismetSystemLibrary.Delay` 5.0)
      (set `FloatingPawnMovement.MaxSpeed` 1200.0 (`self.FloatingPawnMovement`)))
    (:`2`
      (`KismetSystemLibrary.Delay` 5.0)
      (set `self.Damage` 5.0))))

(event `self.ReceiveAnyDamage`
  (params (Damage :type "Float (single-precision)") (DamageType :type "DamageType Object Reference") (InstigatedBy :type "Controller Object Reference") (DamageCauser :type "Actor Object Reference"))
  (`self.DamageOnServer` Damage DamageCauser))

(event `SetSpeedOnMulticast`
  (params (`Max Speed` :type "Float (double-precision)"))
  (set `FloatingPawnMovement.MaxSpeed` `Max Speed` (`self.FloatingPawnMovement`)))

(event `SetSpeedOnServer`
  (params (`Max Speed` :type "Float (double-precision)"))
  (`self.SetSpeedOnMulticast` `Max Speed`))

(event `Death`
  (bind _returnvalue (`GameplayStatics.SpawnEmitterAtLocation` "/Game/ParticleSystem/PS_Explosion.PS_Explosion" (`self.K2_GetActorLocation`)))
  (`FXSystemComponent.SetColorParameter` _returnvalue "PrimaryColor" (`self.PrimaryColor`))
  (`FXSystemComponent.SetColorParameter` _returnvalue "SecondryColor" (`self.SecondryColor`))
  (`self.K2_DestroyActor`))

(event `SetScoreOnMulticast`
  (params (`Damage Causer` :type "Actor Object Reference"))
  (bind _asbp_space_ship_online (cast `/Game/Buleprints/BP_SpaceShip_Online` `Damage Causer`)
    (:`then`
      (set `/Game/Buleprints/BP_SpaceShip_Online.Score` (+ (`/Game/Buleprints/BP_SpaceShip_Online.Score` _asbp_space_ship_online) 100) _asbp_space_ship_online))
    (:`CastFailed`
      (bind _asbp_ai (cast `/Game/Buleprints/BP_AI` `Damage Causer`))
      (set `/Game/Buleprints/BP_AI.Score` (+ (`/Game/Buleprints/BP_AI.Score` _asbp_ai) 100) _asbp_ai))))

(event `DamageOnMulticast`
  (params (HP :type "Float (double-precision)") (`Damage Causer` :type "Actor Object Reference") (Death :type Boolean))
  (bind _output_get (set `self.HP` HP))
  (bind _foundwidgets (`WidgetBlueprintLibrary.GetAllWidgetsOfClass` "/Game/Buleprints/Widget/WBP_HP.WBP_HP_C"))
  (if true
    (`/Game/Buleprints/Widget/WBP_HP.Recieve Damage` (`|GetArrayItem` _foundwidgets) _output_get (`self.BodyColorIndex`) `Damage Causer`)
    (else
      (bind _foundwidgets_2 (`WidgetBlueprintLibrary.GetAllWidgetsOfClass` "/Game/Buleprints/Widget/WBP_HP_Local.WBP_HP_Local_C"))
      (`/Game/Buleprints/Widget/WBP_HP_Local.Recieve Damage` (`|GetArrayItem` _foundwidgets_2) (`self.HP`) (`self.BodyColorIndex`) `Damage Causer`)))
  (bind _returnvalue (`GameplayStatics.SpawnEmitterAtLocation` "/Game/ParticleSystem/PS_Explosion.PS_Explosion" (`self.K2_GetActorLocation`) (struct) (0.5 0.5 0.5)))
  (`FXSystemComponent.SetColorParameter` _returnvalue "PrimaryColor" (struct :`R` 1.0 :`A` 1.0))
  (`FXSystemComponent.SetColorParameter` _returnvalue "SecondryColor" (struct :`R` 0.196078 :`G` 0.129412 :`B` 0.129412 :`A` 1.0))
  (if Death
    (bind _returnvalue_2 (`GameplayStatics.SpawnEmitterAtLocation` "/Game/ParticleSystem/PS_Explosion.PS_Explosion" (`self.K2_GetActorLocation`)))
    (`FXSystemComponent.SetColorParameter` _returnvalue_2 "PrimaryColor" (`self.PrimaryColor`))
    (`FXSystemComponent.SetColorParameter` _returnvalue_2 "SecondryColor" (`self.SecondryColor`))))

(event `DamageOnServer`
  (params (Damage :type "Float (double-precision)") (`Damage Causer` :type "Actor Object Reference"))
  (bind _output_get (set `self.HP` (`KismetMathLibrary.FMin` (- (`self.HP`) Damage) 100.0)))
  (bind _returnvalue (<= _output_get 0.0))
  (if _returnvalue
    (`self.SetScoreOnMulticast` `Damage Causer`)
    (`self.Death`))
  (`self.DamageOnMulticast` _output_get `Damage Causer` _returnvalue))

(event `AIFarAwayMovement`
  ;[1 1 1] AI Movement
  (bind _returnvalue (`KismetSystemLibrary.K2_SetTimerDelegate` (delegate `Loop`) 0.2 true))
  (set `self.AIFarAway_Handle` _returnvalue))

(event `Loop`
  (bind _returnvalue (`self.K2_GetActorLocation`))
  ;[1 1 1] AI Movement
  (bind (_outhits _returnvalue_2) (`KismetSystemLibrary.SphereTraceMultiForObjects` _returnvalue (+ _returnvalue (0.0 0.0 10.0)) 700.0 (`|MakeArray` "ObjectTypeQuery3" :!type "EObjectTypeQuery Enum")))
  (if _returnvalue_2
    (`|AIMoveTo` self (`NavigationSystemV1.K2_GetRandomLocationInNavigableRadius` (+ (* (* (`SceneComponent.GetForwardVector` (`self.StaticMesh`)) -1.0) (`KismetMathLibrary.RandomFloatInRange` 1500.0 2000.0)) (`self.K2_GetActorLocation`)) (`KismetMathLibrary.RandomFloatInRange` 2000.0 2500.0) null null) null 5.0 true)))

(event `AIRandomMovement`
  ;[1 1 1] AI Movement
  (bind _returnvalue (`KismetSystemLibrary.K2_SetTimerDelegate` (delegate `Loop2`) 0.5 true))
  (set `self.AIRandom_Handle` _returnvalue))

(event `Loop2`
  ;[1 1 1] AI Movement
  ;;[1 1 1] 随机移动
  (`|AIMoveTo` self (`NavigationSystemV1.K2_GetRandomLocationInNavigableRadius` (`self.K2_GetActorLocation`) (`KismetMathLibrary.RandomFloatInRange` 1500.0 3000.0) null null) null 5.0 true))

(event `FindItems`
  ;[1 1 1] AI Movement
  (bind _returnvalue (`KismetSystemLibrary.K2_SetTimerDelegate` (delegate `Loop3`) 0.5 true))
  (set `self.FindItem_Handle` _returnvalue))

(event `Loop3`
  (bind (_cloesttarget _items) (`self.FindNestItem`))
  ;[1 1 1] AI Movement
  (`/Engine/EditorBlueprintResources/StandardMacros.IsValid` _items
    (:`Is Valid`
      (if (== self _cloesttarget)
        (`KismetSystemLibrary.K2_ClearAndInvalidateTimerHandle` (`self.AIFarAway_Handle`))
        (`KismetSystemLibrary.K2_ClearAndInvalidateTimerHandle` (`self.AIRandom_Handle`))
        (`|AIMoveTo` self (`self.K2_GetActorLocation` (`.Items` (`self.FindNestItem`))) null 0.0
          (:`then`
            (`self.AIRandomMovement` self)
            (`self.AIFarAwayMovement` self)))))))

(fn `FindNestItem`
  (returns (CloestTarget :type "/Game/Buleprints/BP_AI Object Reference") (Items :type "Actor Object Reference"))
  (locals (LocalItems :type "Actor Object Reference") (LocalArray :type "Array of Float (double-precision)"))
  (bind _returnvalue (`self.K2_GetActorLocation`))
  (`KismetArrayLibrary.Array_Clear` (`local.LocalArray`))
  (bind (_outhit _returnvalue_2) (`KismetSystemLibrary.SphereTraceSingle` _returnvalue (+ _returnvalue (0.0 0.0 10.0)) 4000.0 "TraceTypeQuery4"))
  (if _returnvalue_2
    (bind (_bblockinghit _binitialoverlap _time _distance _location _impactpoint _normal _impactnormal _physmat _hitactor) (`GameplayStatics.BreakHitResult` _outhit))
    (bind _asbp_enemy (cast `/Game/Buleprints/BP_Item` _hitactor)
      (:`then`
        (set `local.LocalItems` _asbp_enemy))
      (:`CastFailed`
        (bind _asbp_enemy_online (cast `/Game/Buleprints/BP_Item_Online` _hitactor))
        (set `local.LocalItems` _asbp_enemy_online)))
    (bind _outactors (`GameplayStatics.GetAllActorsOfClass` "BP_AI_C"))
    (for _array_element _outactors
      (`KismetArrayLibrary.Array_Add` (`local.LocalArray`) (`KismetMathLibrary.Vector_Distance` (`self.K2_GetActorLocation` (`local.LocalItems`)) (`self.K2_GetActorLocation` _array_element))))
    (return (`|GetArrayItem` _outactors (`KismetMathLibrary.MinOfFloatArray` (`local.LocalArray`))) (`local.LocalItems`))))

(fn `Fire`
  (bind (_returnvalue_location _returnvalue_rotation) (`KismetMathLibrary.BreakTransform` (`SceneComponent.K2_GetComponentToWorld` (`self.Scene`))))
  (`|SpawnActorFromClass` "/Game/Buleprints/BP_Bullet.BP_Bullet_C" (`KismetMathLibrary.MakeTransform` _returnvalue_location _returnvalue_rotation) "Undefined" "OverrideRootScale" null (`self.Damage`) self (`self.PrimaryColor`) null)
  (`GameplayStatics.PlaySoundAtLocation` "/Game/Sound/Shoot_Cue.Shoot_Cue" _returnvalue_location (struct) 0.75 1.0 0.0 "/Game/Sound/SoundAttenuation.SoundAttenuation" null null))

(fn `Get Index`
  (bind (_lefts _rights _returnvalue) (`KismetStringLibrary.Split` (`KismetSystemLibrary.GetObjectName` self) "AI"))
  (if _returnvalue
    (if (`KismetStringLibrary.EqualEqual_StrStr` _rights "_2")
      (set `self.BodyColorIndex` 1)
      (return)
      (else
        (set `self.BodyColorIndex` (`KismetStringLibrary.Conv_StringToInt` _rights))
        (return)))
    (else
      (return))))

(fn `Get WBP_Main`
  (returns (Output_Get :type "UserWidget Object Reference"))
  (bind _foundwidgets (`WidgetBlueprintLibrary.GetAllWidgetsOfClass` "/Game/Buleprints/Widget/WBP_HP.WBP_HP_C"))
  (if (> (`KismetArrayLibrary.Array_Length` _foundwidgets) 0)
    (set `self.WBP_HP` (`|GetArrayItem` _foundwidgets))
    (return null)
    (else
      (bind _foundwidgets_2 (`WidgetBlueprintLibrary.GetAllWidgetsOfClass` "/Game/Buleprints/Widget/WBP_HP_Local.WBP_HP_Local_C"))
      (return null))))

(fn `UserConstructionScript`)