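; Online spawner Blueprint that, despite its enemy-spawn name, repeatedly spawns BP_Item_Online actors at random points around itself.
; CustomBeginplay calls SpawnOnServer, which loops endlessly with a DurationTime delay between spawns.
; Each item lands within half the Box component's scaled extent around the actor's location, with a flattened Z scale and a random body color index.
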(event `Custom Beginplay`
  (`self.SpawnOnServer`))

(event `SpawnOnServer`
  (`|SpawnActorFromClass` "/Game/Buleprints/BP_Item_Online.BP_Item_Online_C" (`KismetMathLibrary.MakeTransform` (`KismetMathLibrary.RandomPointInBoundingBox` (`self.K2_GetActorLocation`) (/ (`BoxComponent.GetScaledBoxExtent` (`self.Box`)) 2.0)) (struct) (1.0 1.0 0.1)) "Undefined" "OverrideRootScale" null (`KismetMathLibrary.RandomIntegerInRange` 0 3) null :!label _label)
  (`KismetSystemLibrary.Delay` (`self.DurationTime`))
  (goto _label))

(fn `UserConstructionScript`)