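; Networked pickup whose BodyColorIndex sets both its color and its effect: speed boost, health change through ApplyDamage, damage buff or score.
; BeginPlay tints a dynamic material and plays a scale Timeline through server-to-multicast-named events.
; Overlaps apply the effect to AI ships via OverlapOnMulticast but to player ships inline, with score shown through player controller 0's HUD.
; Each pickup then spawns a color-matched explosion and destroys itself.
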(event `self.ReceiveBeginPlay`
  (bind _foundwidgets (`WidgetBlueprintLibrary.GetAllWidgetsOfClass` "/Game/Buleprints/Widget/WBP_HP.WBP_HP_C"))
  (set `self.WBP_HP` (`|GetArrayItem` _foundwidgets))
  (`self.SetColorOnSever`))

(event `SetColorOnSever`
  (`self.SetColorOnMulticast`))

(event `SetColorOnMulticast`
  (bind _returnvalue (select `int` (`self.BodyColorIndex`) :`0` (struct :`R` 1.0 :`G` 0.538341 :`A` 1.0) :`1` (struct :`G` 1.0 :`A` 1.0) :`2` (struct :`R` 1.0 :`A` 1.0) :`3` (struct :`A` 1.0) :!type "LinearColor Structure"))
  (bind _returnvalue_2 (`KismetMaterialLibrary.CreateDynamicMaterialInstance` "/Game/SpaceshipBattle/Materials/M_Base_Ship.M_Base_Ship"))
  (`MaterialInstanceDynamic.SetVectorParameterValue` _returnvalue_2 "Color3" _returnvalue)
  (set `self.PrimaryColor` _returnvalue)
  (set `self.SecondryColor` _returnvalue)
  (`PrimitiveComponent.SetMaterial` (`self.Enemy SM`) 0 _returnvalue_2)
  (bind (_direction _scale) (`Timeline|Timeline_0`)
    (:`Update`
      (`self.SetActorScale3D` (`KismetMathLibrary.Conv_DoubleToVector` _scale)))))

(event `On Death`
  (`self.DeathOnMulticast`))

(event `DeathOnMulticast`
  (bind _returnvalue (`GameplayStatics.SpawnEmitterAtLocation` "/Game/ParticleSystem/PS_Explosion.PS_Explosion" (`self.K2_GetActorLocation`)))
  (`FXSystemComponent.SetColorParameter` _returnvalue "PrimaryColor" (`self.PrimaryColor`))
  (`FXSystemComponent.SetColorParameter` _returnvalue "SecondryColor" (`self.SecondryColor`))
  (`self.K2_DestroyActor`))

(event `OverlapOnMulticast`
  (params (`As AI` :type "/Game/Buleprints/BP_AI Object Reference"))
  (bind _as_ai (`self.As AI`))
  (bind _as_ai_2 (`self.As AI`))
  (bind _as_ai_3 (`self.As AI`))
  (set `self.As AI` `As AI`)
  (switch `int` (`self.BodyColorIndex`)
    (:`0`
      (`/Game/Buleprints/BP_AI.SetSpeedOnServer` _as_ai_2 2400.0)
      (`/Game/Buleprints/BP_AI.BufferDisapper` _as_ai_2 (`self.BodyColorIndex`))
      (`self.On Death`))
    (:`1`
      (`GameplayStatics.ApplyDamage` (`self.As AI`) (`self.HealthAdd`))
      (`self.On Death`))
    (:`2`
      (set `/Game/Buleprints/BP_AI.Damage` (`self.DamageBuffer`) _as_ai)
      (`/Game/Buleprints/BP_AI.BufferDisapper` _as_ai (`self.BodyColorIndex`))
      (`self.On Death`))
    (:`3`
      (bind _asbp_login_player_controller (cast `/Game/Buleprints/BP_LoginPlayerController` (`GameplayStatics.GetPlayerController` 0)))
      (bind _output_get (set `/Game/Buleprints/BP_AI.Score` (+ (`/Game/Buleprints/BP_AI.Score` _as_ai_3) 50) _as_ai_3))
      (`/Game/Buleprints/Widget/WBP_Score.Get Score` (`|GetArrayItem` (`/Game/Buleprints/Widget/WBP_HP.GetScoreArray` (`/Game/Buleprints/BP_LoginPlayerController.WBP_HP` _asbp_login_player_controller)) (`/Game/Buleprints/BP_AI.BodyColorIndex` _as_ai_3)) _output_get)
      (`self.On Death`))))

(event `self.ReceiveActorBeginOverlap`
  (params (OtherActor :type "Actor Object Reference"))
  (bind _as_bp_space_ship_online (`self.As BP Space Ship Online`))
  (bind _as_bp_space_ship_online_2 (`self.As BP Space Ship Online`))
  (bind _as_bp_space_ship_online_3 (`self.As BP Space Ship Online`))
  (bind _asbp_ai (cast `/Game/Buleprints/BP_AI` OtherActor)
    (:`then`
      (`self.OverlapOnMulticast` _asbp_ai))
    (:`CastFailed`
      (bind _asbp_space_ship_online (cast `/Game/Buleprints/BP_SpaceShip_Online` OtherActor))
      (set `self.As BP Space Ship Online` _asbp_space_ship_online)
      (switch `int` (`self.BodyColorIndex`)
        (:`0`
          (`/Game/Buleprints/BP_SpaceShip_Online.Set Movement Speed On Server` _as_bp_space_ship_online 5000.0)
          (`/Game/Buleprints/BP_SpaceShip_Online.BufferDisapper` _as_bp_space_ship_online (`self.BodyColorIndex`))
          (`self.On Death`))
        (:`1`
          (`GameplayStatics.ApplyDamage` (`self.As BP Space Ship Online`) (`self.HealthAdd`))
          (`self.On Death`))
        (:`2`
          (set `/Game/Buleprints/BP_SpaceShip_Online.Damage` (`self.DamageBuffer`) _as_bp_space_ship_online_3)
          (`/Game/Buleprints/BP_SpaceShip_Online.BufferDisapper` _as_bp_space_ship_online_3 (`self.BodyColorIndex`))
          (`self.On Death`))
        (:`3`
          (bind _asbp_login_player_controller (cast `/Game/Buleprints/BP_LoginPlayerController` (`GameplayStatics.GetPlayerController` 0)))
          (bind _output_get (set `/Game/Buleprints/BP_SpaceShip_Online.Score` (+ (`/Game/Buleprints/BP_SpaceShip_Online.Score` _as_bp_space_ship_online_2) 50) _as_bp_space_ship_online_2))
          (`/Game/Buleprints/Widget/WBP_Score.Get Score` (`|GetArrayItem` (`/Game/Buleprints/Widget/WBP_HP.GetScoreArray` (`/Game/Buleprints/BP_LoginPlayerController.WBP_HP` _asbp_login_player_controller)) (`/Game/Buleprints/BP_SpaceShip_Online.BodyIndex` _as_bp_space_ship_online_2)) _output_get)
          (`self.On Death`))))))

(fn `UserConstructionScript`)