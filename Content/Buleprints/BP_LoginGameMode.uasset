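; Game mode for an online spaceship match that runs the player lobby, match start, damage updates and game end.
; Parallel arrays track controllers, local Steam persona names, ready and death flags, pushing lobby changes to every controller.
; Start spawns and possesses a ship per player at TargetPoints, filling slots up to four with AI.
; Damage updates reach all controllers, which are told to stop once every death flag is true.
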(event `self.K2_PostLogin`
  (params (NewPlayer :type "PlayerController Object Reference"))
  (`KismetArrayLibrary.Array_Add` (`self.Death`))
  (`KismetArrayLibrary.Array_Add` (`self.Ready`))
  (bind _returnvalue (`AdvancedSteamFriendsLibrary.GetSteamPersonaName` (`AdvancedSteamFriendsLibrary.GetLocalSteamIDFromSteam`)))
  (`KismetArrayLibrary.Array_Add` (`self.Username`) (`KismetTextLibrary.Conv_StringToText` _returnvalue))
  (bind _asbp_login_player_controller (cast `/Game/Buleprints/BP_LoginPlayerController` NewPlayer))
  (`KismetArrayLibrary.Array_Add` (`self.Login Player Controller`) _asbp_login_player_controller)
  (`self.UpdateVarOnClient`))

(event `self.K2_OnLogout`
  (params (ExitingController :type "Controller Object Reference"))
  (bind _login_player_controller (`self.Login Player Controller`))
  (`KismetSystemLibrary.Delay` 0.1)
  (bind _asbp_login_player_controller (cast `/Game/Buleprints/BP_LoginPlayerController` ExitingController))
  (bind _returnvalue (`KismetArrayLibrary.Array_Find` _login_player_controller _asbp_login_player_controller))
  (`KismetArrayLibrary.Array_Remove` (`self.Ready`) _returnvalue)
  (`KismetArrayLibrary.Array_Remove` (`self.Username`) _returnvalue)
  (`KismetArrayLibrary.Array_RemoveItem` _login_player_controller _asbp_login_player_controller)
  (`self.UpdateVarOnClient`))

(event `UpdateVarOnClient`
  (if (`KismetArrayLibrary.Array_IsValidIndex` (`self.Login Player Controller`))
    (for _array_element (`self.Login Player Controller`)
      (`/Game/Buleprints/BP_LoginPlayerController.UpdateInfoOnClient` _array_element (`self.Username`) (`self.Ready`)))))

(event `UpdateOnReady`
  (params (PlayerController :type "/Game/Buleprints/BP_LoginPlayerController Object Reference (by ref)") (Ready :type Boolean))
  (bind _login_player_controller (`self.Login Player Controller`))
  (bind _returnvalue (`KismetArrayLibrary.Array_Find` _login_player_controller PlayerController))
  (if (`KismetArrayLibrary.Array_IsValidIndex` _login_player_controller _returnvalue)
    (`KismetArrayLibrary.Array_Set` (`self.Ready`) _returnvalue Ready)
    (`self.UpdateVarOnClient`)))

(event `StartGameOnClient`
  (bind _login_player_controller (`self.Login Player Controller`))
  (for (_array_element _array_index) _login_player_controller
    (bind _outactors (`GameplayStatics.GetAllActorsOfClass` "/Script/Engine.TargetPoint"))
    (bind _returnvalue (`|SpawnActorFromClass` "/Game/Buleprints/BP_SpaceShip_Online.BP_SpaceShip_Online_C" (`KismetMathLibrary.Conv_VectorToTransform` (`self.K2_GetActorLocation` (`|GetArrayItem` _outactors _array_index))) "Undefined" "OverrideRootScale" null _array_index null))
    (`Controller.Possess` _array_element _returnvalue)
    (`/Game/Buleprints/BP_LoginPlayerController.OpenGameOnClient` _array_element))
  (if (< (`KismetArrayLibrary.Array_Length` _login_player_controller) 4)
    (for _index (range (+ (`KismetArrayLibrary.Array_LastIndex` _login_player_controller) 1) 4)
      (bind _outactors_2 (`GameplayStatics.GetAllActorsOfClass` "/Script/Engine.TargetPoint"))
      (`|SpawnActorFromClass` "/Game/Buleprints/BP_AI.BP_AI_C" (`KismetMathLibrary.Conv_VectorToTransform` (`self.K2_GetActorLocation` (`|GetArrayItem` _outactors_2 _index))) "Undefined" "OverrideRootScale" null _index null))))

(event `ReceiveDamageUIOnClient`
  (params (HP :type "Float (double-precision)") (Index :type Integer) (`Damage Target` :type "Actor Object Reference"))
  (for _array_element (`self.Login Player Controller`)
    (`/Game/Buleprints/BP_LoginPlayerController.ReceiveDamage` _array_element HP Index `Damage Target`)))

(event `StopGameOnClient`
  (params (Death :type Boolean) (ItemToFind :type "/Game/Buleprints/BP_LoginPlayerController Object Reference (by ref)"))
  (bind _login_player_controller (`self.Login Player Controller`))
  (bind _returnvalue (`KismetArrayLibrary.Array_Find` _login_player_controller ItemToFind))
  (if (`KismetArrayLibrary.Array_IsValidIndex` _login_player_controller _returnvalue)
    (`KismetArrayLibrary.Array_Set` (`self.Death`) _returnvalue Death)
    (if (not (`KismetArrayLibrary.Array_Contains` (`self.Death`)))
      (for _array_element (`self.Login Player Controller`)
        (`/Game/Buleprints/BP_LoginPlayerController.StopGameOnController` _array_element true)))))

(fn `UserConstructionScript`)