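; BP_GameMode is a game mode Blueprint that detects the player's victory.
; A looping timer started on BeginPlay repeatedly counts BP_SpaceShip and BP_AI actors in the level.
; When at most one ship or AI remains and no AI is left, it calls GameOver with "Victory" on the first BP_SpaceShip and clears the timer.
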(event `self.ReceiveBeginPlay`
  (bind _returnvalue (`KismetSystemLibrary.K2_SetTimerDelegate` (delegate `Loop`) 0.1 true))
  (set `self.TimerHandle` _returnvalue))

(event `Loop`
  (bind _outactors (`GameplayStatics.GetAllActorsOfClass` "/Game/Buleprints/BP_SpaceShip.BP_SpaceShip_C"))
  (set `self.Player` (`KismetArrayLibrary.Array_Length` _outactors))
  (bind _outactors_2 (`GameplayStatics.GetAllActorsOfClass` "/Game/Buleprints/BP_AI.BP_AI_C"))
  (set `self.AI` (`KismetArrayLibrary.Array_Length` _outactors_2))
  (if (<= (+ (`self.AI`) (`self.Player`)) 1)
    (if (== (`self.AI`) 0)
      (bind _outactors_3 (`GameplayStatics.GetAllActorsOfClass` "/Game/Buleprints/BP_SpaceShip.BP_SpaceShip_C"))
      (`/Game/Buleprints/BP_SpaceShip.GameOver` (`|GetArrayItem` _outactors_3) "Victory")
      (`KismetSystemLibrary.K2_ClearAndInvalidateTimerHandle` (`self.TimerHandle`)))))

(fn `UserConstructionScript`)