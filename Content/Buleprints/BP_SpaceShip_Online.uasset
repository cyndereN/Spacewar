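; Player spaceship Character for an online shooter against other ships and BP_AI, with axis movement and controller-driven rotation.
; Server-to-multicast event pairs handle looping timer fire of BP_Bullet, speed changes, body-index coloring and damage.
; Damage updates controller UI and spawns explosions; death awards the killer score, hides the ship and shows game over.
; A looping timer counts visible ships plus AI to declare victory, and BufferDisapper resets speed or damage after a delay.
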(event `InputAxis|MoveForward`
  (params (AxisValue :type "Float (single-precision)"))
  (`self.AddMovementInput` (1.0 0.0 0.0) AxisValue))

(event `InputAxis|MoveRight`
  (params (AxisValue :type "Float (single-precision)"))
  (`self.AddMovementInput` (0.0 1.0 0.0) AxisValue))

(event `ServerControlRotation`
  (bind _returnvalue (`self.GetPlayerControllerServer`))
  (`/Engine/EditorBlueprintResources/StandardMacros.IsValid` _returnvalue
    (:`Is Valid`
      (`Controller.SetControlRotation` _returnvalue (`self.Rotation`)))))

(event `self.ReceiveTick`
  (params (DeltaSeconds :type "Float (single-precision)"))
  (bind _asbp_login_player_controller (cast `/Game/Buleprints/BP_LoginPlayerController` (`GameplayStatics.GetPlayerController` 0)))
  (bind _output_get (`/Game/Buleprints/BP_LoginPlayerController.SetPlayerController` _asbp_login_player_controller))
  (set `self.Rotation` _output_get)
  (`self.ServerControlRotation`)
  (`self.ClientControlRotation`))

(event `ClientControlRotation`
  (bind _returnvalue (`self.GetPlayerControllerServer`))
  (`/Engine/EditorBlueprintResources/StandardMacros.IsValid` _returnvalue
    (:`Is Valid`
      (`Controller.SetControlRotation` _returnvalue (`self.Rotation`)))))

(event `EndFireOnMulticast`
  (`KismetSystemLibrary.K2_ClearAndInvalidateTimerHandle` (`self.Handle`)))

(event `EndFireOnServer`
  (`self.EndFireOnMulticast`))

(event `StartFireOnServer`
  (`self.StartFireOnMulticast`))

(event `StartFireOnMulticast`
  (bind _returnvalue (`KismetSystemLibrary.K2_SetTimerDelegate` (delegate `Loop`) 0.2 true))
  (set `self.Handle` _returnvalue))

(event `Loop`
  (bind (_returnvalue_location _returnvalue_rotation) (`KismetMathLibrary.BreakTransform` (`SceneComponent.K2_GetComponentToWorld` (`self.Scene`))))
  (set `self.Return Value Location` _returnvalue_location)
  (set `self.Return Value Rotation` _returnvalue_rotation)
  (`self.Fire` (`self.Return Value Location`) (`self.Return Value Rotation`)))

(event `InputAction|Fire`
  (params (Key :type "Key Structure"))
  (:`Pressed`
    (`self.StartFireOnServer`))
  (:`Released`
    (`self.EndFireOnServer`)))

(event `Set Movement Speed On Server`
  (params (`Max Walk Speed` :type "Float (double-precision)"))
  (`self.Set Movement Speed On Multicast` `Max Walk Speed`))

(event `Set Movement Speed On Multicast`
  (params (`Max Walk Speed` :type "Float (double-precision)"))
  (set `CharacterMovementComponent.MaxWalkSpeed` `Max Walk Speed` (`self.CharacterMovement`)))

(event `VictoryOnServer`
  (bind _returnvalue (`KismetSystemLibrary.K2_SetTimerDelegate` (delegate `Victory`) 0.5 true))
  (set `self.TimerHandle` _returnvalue))

(event `BufferDisapper`
  (params (Int :type Integer))
  (switch `int` Int
    (:`0`
      (`KismetSystemLibrary.Delay` 5.0)
      (`self.Set Movement Speed On Server` 2500.0))
    (:`2`
      (`KismetSystemLibrary.Delay` 5.0)
      (set `self.Damage` 5.0))))

(event `self.ReceiveBeginPlay`
  (`self.SetColorOnServer`)
  (`self.VictoryOnServer`))

(event `SetColorOnServer`
  (`self.SetColorMulticast`))

(event `Victory`
  (`self.GetPlayerLength`))

(event `SetColorMulticast`
  (bind _returnvalue (select `int` (`self.BodyIndex`) :`0` (struct :`R` 1.0 :`A` 1.0) :`1` (struct :`G` 1.0 :`A` 1.0) :`2` (struct :`B` 1.0 :`A` 1.0) :`3` (struct :`R` 1.0 :`G` 1.0 :`A` 1.0) :!type "LinearColor Structure"))
  (bind _returnvalue_2 (`KismetMaterialLibrary.CreateDynamicMaterialInstance` "/Game/SpaceshipBattle/Materials/MI_Ship_Player.MI_Ship_Player"))
  (`MaterialInstanceDynamic.SetVectorParameterValue` _returnvalue_2 "Color3" _returnvalue)
  (set `self.PrimaryColor` _returnvalue)
  (`PrimitiveComponent.SetMaterial` (`self.StaticMesh`) 0 _returnvalue_2))

(event `Key|Tab`
  (params (Key :type "Key Structure")))

(event `Key|Escape`
  (params (Key :type "Key Structure")))

(event `Death`
  (`self.GameOver` "GameOver"))

(event `SetScoreOnMulticast`
  (params (`Damage Causer` :type "Actor Object Reference"))
  (bind _asbp_space_ship_online (cast `/Game/Buleprints/BP_SpaceShip_Online` `Damage Causer`)
    (:`then`
      (set `/Game/Buleprints/BP_SpaceShip_Online.Score` (+ (`/Game/Buleprints/BP_SpaceShip_Online.Score` _asbp_space_ship_online) 100) _asbp_space_ship_online))
    (:`CastFailed`
      (bind _asbp_ai (cast `/Game/Buleprints/BP_AI` `Damage Causer`))
      (set `/Game/Buleprints/BP_AI.Score` (+ (`/Game/Buleprints/BP_AI.Score` _asbp_ai) 100) _asbp_ai))))

(event `self.ReceiveAnyDamage`
  (params (Damage :type "Float (single-precision)") (DamageType :type "DamageType Object Reference") (InstigatedBy :type "Controller Object Reference") (DamageCauser :type "Actor Object Reference"))
  (`self.DamageOnServer` Damage DamageCauser))

(event `DamageOnServer`
  (params (Damage :type "Float (double-precision)") (`Damage Causer` :type "Actor Object Reference"))
  (bind _output_get (set `self.HP` (`KismetMathLibrary.FMin` (- (`self.HP`) Damage) 100.0)))
  (bind _returnvalue (<= _output_get 0.0))
  (if _returnvalue
    (`self.SetScoreOnMulticast` `Damage Causer`)
    (`self.Death`))
  (`self.DamageOnMulticast` _output_get `Damage Causer` _returnvalue))

(event `DamageOnMulticast`
  (params (HP :type "Float (double-precision)") (`Damage Causer` :type "Actor Object Reference") (Death :type Boolean))
  (bind _asbp_login_player_controller (cast `/Game/Buleprints/BP_LoginPlayerController` (`GameplayStatics.GetPlayerController` 0)))
  (`/Game/Buleprints/BP_LoginPlayerController.ReceiveDamageUIOnServer` _asbp_login_player_controller HP (`self.BodyIndex`) `Damage Causer`)
  (bind _returnvalue (`GameplayStatics.SpawnEmitterAtLocation` "/Game/ParticleSystem/PS_Explosion.PS_Explosion" (`self.K2_GetActorLocation`) (struct) (0.5 0.5 0.5)))
  (`FXSystemComponent.SetColorParameter` _returnvalue "PrimaryColor" (struct :`R` 20.0 :`G` 16.684612 :`A` 1.0))
  (`FXSystemComponent.SetColorParameter` _returnvalue "SecondryColor" (struct :`R` 7.491335 :`G` 10.0 :`B` 9.800827 :`A` 1.0))
  (if Death
    (bind _returnvalue_2 (`GameplayStatics.SpawnEmitterAtLocation` "/Game/ParticleSystem/PS_Explosion.PS_Explosion" (`self.K2_GetActorLocation`)))
    (`FXSystemComponent.SetColorParameter` _returnvalue_2 "PrimaryColor" (`self.PrimaryColor`))
    (`FXSystemComponent.SetColorParameter` _returnvalue_2 "SecondryColor" (`self.SecondryColor`))
    (`SceneComponent.SetVisibility` (`self.StaticMesh`) false false)
    (`self.SetActorEnableCollision` self false)))

(fn `Fire`
  (params (`Spawn Transform Location` :type "Vector Structure") (`Spawn Transform Rotation` :type "Rotator Structure"))
  (locals (LocalLocation :type "Vector Structure" :default (0.0 0.0 0.0)))
  (bind _returnvalue_location (`KismetMathLibrary.BreakTransform` (`SceneComponent.K2_GetComponentToWorld` (`self.Scene`))))
  (`|SpawnActorFromClass` "/Game/Buleprints/BP_Bullet.BP_Bullet_C" (`KismetMathLibrary.MakeTransform` `Spawn Transform Location` `Spawn Transform Rotation`) "Undefined" "OverrideRootScale" null (`self.Damage`) self (`self.PrimaryColor`) null)
  (`GameplayStatics.PlaySoundAtLocation` "/Game/Sound/Shoot_Cue.Shoot_Cue" _returnvalue_location (struct) 0.75 1.0 0.0 "/Game/Sound/SoundAttenuation.SoundAttenuation" null null))

(fn `GameOver`
  (params (Text :type Text))
  (bind _returnvalue (`|CreateWidget` "/Game/Buleprints/Widget/WBP_GameOver.WBP_GameOver_C" null Text))
  (`UserWidget.AddToViewport` _returnvalue 0)
  (`self.EndFireOnMulticast`)
  (`self.DisableInput` self (`GameplayStatics.GetPlayerController` 0))
  (return))

(fn `GetPlayerControllerServer`
  (returns (ReturnValue :type "PlayerController Object Reference"))
  (return (`GameplayStatics.GetPlayerController` 0)))

(fn `GetPlayerLength`
  (locals (AiLen :type Integer :default 0) (PlayerLen :type Integer :default 0))
  (bind _outactors (`GameplayStatics.GetAllActorsOfClass` "/Game/Buleprints/BP_AI.BP_AI_C"))
  (set `local.AiLen` (`KismetArrayLibrary.Array_Length` _outactors))
  (set `local.PlayerLen` 0)
  (bind _outactors_2 (`GameplayStatics.GetAllActorsOfClass` "BP_SpaceShip_Online_C"))
  (for _array_element _outactors_2
    (set `local.PlayerLen` (+ (`local.PlayerLen`) (`KismetMathLibrary.Conv_BoolToInt` (`SceneComponent.IsVisible` (`/Game/Buleprints/BP_SpaceShip_Online.StaticMesh` _array_element))))))
  (if (<= (+ (`local.PlayerLen`) (`local.AiLen`)) 1)
    (if (== (`local.PlayerLen`) 1)
      (bind _returnvalue (`|CreateWidget` "/Game/Buleprints/Widget/WBP_GameOver.WBP_GameOver_C" null "Victory"))
      (`UserWidget.AddToViewport` _returnvalue 0)
      (`KismetSystemLibrary.K2_ClearAndInvalidateTimerHandle` (`self.TimerHandle`)))))

(fn `SetControlRotation`
  (bind _returnvalue (`GameplayStatics.GetPlayerController` (`KismetStringLibrary.Conv_StringToInt` (`KismetStringLibrary.Right` (`KismetSystemLibrary.GetDisplayName` self) 1))))
  (bind (_locationx _locationy) (`PlayerController.GetMousePosition` _returnvalue))
  (bind (_returnvalue_roll _returnvalue_pitch _returnvalue_yaw) (`KismetMathLibrary.BreakRotator` (`KismetMathLibrary.FindLookAtRotation` (`KismetMathLibrary.Conv_Vector2DToVector` (/ (`WidgetLayoutLibrary.GetViewportSize`) 2.0)) (`KismetMathLibrary.Conv_Vector2DToVector` (`KismetMathLibrary.MakeVector2D` _locationx _locationy)))))
  (`/Engine/EditorBlueprintResources/StandardMacros.IsValid` _returnvalue
    (:`Is Valid`
      (set `self.Rotation` (`KismetMathLibrary.MakeRotator` _returnvalue_roll _returnvalue_pitch (+ _returnvalue_yaw 90.0)))
      (return))))

(fn `UserConstructionScript`)