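; BP_SpaceShip is the player's ship: it fires bullets, takes damage and ends the game when destroyed.
; Holding Fire runs a looping timer that spawns colored BP_Bullet actors with sound at the spawn point.
; Damage updates an HP widget and spawns tinted explosions; at zero HP it shows game over, disables input and hides the ship.
; BufferDisapper resets speed or damage after a delay, while Tab or Escape opens an interface widget.
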(event `EndFire`
  (`KismetSystemLibrary.K2_ClearAndInvalidateTimerHandle` (`self.Handle`)))

(event `StartFire`
  (bind _returnvalue (`KismetSystemLibrary.K2_SetTimerDelegate` (delegate `Loop`) 0.2 true))
  (set `self.Handle` _returnvalue))

(event `Loop`
  (bind (_returnvalue_location _returnvalue_rotation) (`KismetMathLibrary.BreakTransform` (`SceneComponent.K2_GetComponentToWorld` (`self.SpawnPoint`))))
  (`|SpawnActorFromClass` "/Game/Buleprints/BP_Bullet.BP_Bullet_C" (`KismetMathLibrary.MakeTransform` _returnvalue_location _returnvalue_rotation) "Undefined" "OverrideRootScale" null (`self.Damage`) self (`self.PrimaryColor`) null)
  (`GameplayStatics.PlaySoundAtLocation` "/Game/Sound/Shoot_Cue.Shoot_Cue" _returnvalue_location (struct) 0.75 1.0 0.0 null null null))

(event `InputAction|Fire`
  (params (Key :type "Key Structure"))
  (:`Pressed`
    (`self.StartFire`))
  (:`Released`
    (`self.EndFire`)))

(event `BufferDisapper`
  (params (Int :type Integer))
  (switch `int` Int
    (:`0`
      (`KismetSystemLibrary.Delay` 5.0)
      (set `self.Speed` 2500.0))
    (:`2`
      (`KismetSystemLibrary.Delay` 5.0)
      (set `self.Damage` 2.0))))

(event `self.ReceiveBeginPlay`
  (bind _returnvalue (`|CreateWidget` "/Game/Buleprints/Widget/WBP_HP_Local.WBP_HP_Local_C"))
  (bind _output_get (set `self.WBP_HP` _returnvalue))
  (`UserWidget.AddToViewport` _output_get 0))

(event `Key|Tab`
  (params (Key :type "Key Structure"))
  (:`Pressed`
    (bind _returnvalue (`|CreateWidget` "/Game/Buleprints/Widget/WBP_UserInterface.WBP_UserInterface_C" :!label _label))
    (bind _output_get (set `self.Interface` _returnvalue))
    (`UserWidget.AddToViewport` _output_get 0)))

(event `Key|Escape`
  (params (Key :type "Key Structure"))
  (:`Pressed`
    (goto _label)))

(event `Death`
  (`self.GameOver` "GameOver")
  (bind _returnvalue (`GameplayStatics.SpawnEmitterAtLocation` "/Game/ParticleSystem/PS_Explosion.PS_Explosion" (`self.K2_GetActorLocation`)))
  (`FXSystemComponent.SetColorParameter` _returnvalue "PrimaryColor" (`self.PrimaryColor`))
  (`FXSystemComponent.SetColorParameter` _returnvalue "SecondryColor" (`self.SecondryColor`))
  (`SceneComponent.SetVisibility` (`self.ShipSM`) false false)
  (`self.SetActorEnableCollision` false))

(event `self.ReceiveAnyDamage`
  (params (Damage :type "Float (single-precision)") (DamageType :type "DamageType Object Reference") (InstigatedBy :type "Controller Object Reference") (DamageCauser :type "Actor Object Reference"))
  (bind _output_get (set `self.HP` (- (`self.HP`) Damage)))
  (`/Game/Buleprints/Widget/WBP_HP_Local.Recieve Damage` (`self.WBP_HP`) _output_get 0 DamageCauser)
  (bind _returnvalue (`GameplayStatics.SpawnEmitterAtLocation` "/Game/ParticleSystem/PS_Explosion.PS_Explosion" (`self.K2_GetActorLocation`) (struct) (0.5 0.5 0.5)))
  (`FXSystemComponent.SetColorParameter` _returnvalue "PrimaryColor" (struct :`R` 20.0 :`G` 16.684612 :`A` 1.0))
  (`FXSystemComponent.SetColorParameter` _returnvalue "SecondryColor" (struct :`R` 7.491335 :`G` 10.0 :`B` 9.800827 :`A` 1.0))
  (if (<= _output_get 0.0)
    (`self.Death`)))

(fn `GameOver`
  (params (Text :type Text))
  (bind _returnvalue (`|CreateWidget` "/Game/Buleprints/Widget/WBP_GameOver.WBP_GameOver_C" null Text))
  (`UserWidget.AddToViewport` _returnvalue 0)
  (`self.EndFire`)
  (`self.DisableInput` self (`GameplayStatics.GetPlayerController` 0))
  (return))

(fn `UserConstructionScript`)